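; Camera manager that sets up a single shared camera for local players.
; SetUpSharedCamera runs its logic only when the owning player controller has ID 0, so only that player spawns a BP_SharedCamera.
; It stores the spawned camera in CamaraRef and makes it player 0's view target.
; Nothing in this Blueprint calls the event, and Tick and overlap events are disabled.
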(event `SetUpSharedCamera`
  (if (== (`GameplayStatics.GetPlayerControllerID` (`self.GetOwningPlayerController`)) 0)
    (bind _returnvalue (`|SpawnActorFromClass` "/Game/Dynamic/SharedCamera/BP_SharedCamera.BP_SharedCamera_C" (`KismetMathLibrary.MakeTransform` (0.0 0.0 0.0)) "Undefined" "MultiplyWithRoot" null null))
    (set `self.CamaraRef` _returnvalue)
    (`PlayerController.SetViewTargetWithBlend` (`GameplayStatics.GetPlayerController` 0) (`self.CamaraRef`) 0.0 "VTBlend_Linear" 0.0 false)))

(fn `UserConstructionScript`)